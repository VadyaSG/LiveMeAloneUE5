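; GM_LiveMeAlone is a game mode that runs the countdown timer and tracks the score.
; A looping one-second timer started on BeginPlay decrements GameTime.
; When GameTime reaches zero, it clears the timer and sends OnTimerEndMessage to the first player controller.
; AddScore increments Score and broadcasts the OnScoreChanged dispatcher to notify listeners.
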(event Custom|GameTimerEvent
  (bind _result (Math|Integer|DecrementInt (Variables|Default|GetGameTime))
    (:%20%20
      (bind _output_get (Variables|Default|SetGameTime _result))
      (if (== _output_get 0)
        (Utilities|Time|ClearandInvalidateTimerbyHandle (Variables|Default|GetTimerHandleRef))
        (Class|BPIGameModeInfo|OnTimerEnd(Message) (Game|GetPlayerController 0))))))

(event Custom|AddScore
  (bind _result (Math|Integer|IncrementInt (Variables|Default|GetScore))
    (:%20%20
      (Variables|Default|SetScore _result)
      (Default|CallOnScoreChanged))))

(event EventBeginPlay
  (bind _returnvalue (Utilities|Time|SetTimerbyEvent (delegate Custom|GameTimerEvent) 1.0 true))
  (Variables|Default|SetTimerHandleRef _returnvalue))

(fn ConstructionScript)